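; BP_MyHUD creates the on-screen UI for either the lobby or the game and relays score updates to it.
; On BeginPlay it casts the game mode to BP_LobbyGM, adding WBP_Lobby to the viewport on success and WBP_MyGame otherwise.
; AddScore passes the score to the game widget's UpdateText, without checking that this widget was created.
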(event `self.ReceiveBeginPlay`
  (cast `/Game/BP_LobbyGM` (`GameplayStatics.GetGameMode`)
    (:`then`
      (bind _returnvalue (`|CreateWidget` "/Game/UI/WBP_Lobby.WBP_Lobby_C"))
      (bind _output_get (set `self.LobbyWidget` _returnvalue))
      (`UserWidget.AddToViewport` _output_get 0))
    (:`CastFailed`
      (bind _returnvalue_2 (`|CreateWidget` "/Game/UI/WBP_MyGame.WBP_MyGame_C"))
      (bind _output_get_2 (set `self.RefWidget` _returnvalue_2))
      (`UserWidget.AddToViewport` _output_get_2 0))))

(event `AddScore`
  (params (score :type Integer))
  (`/Game/UI/WBP_MyGame.Update Text` (`self.RefWidget`) score))

(fn `UserConstructionScript`)