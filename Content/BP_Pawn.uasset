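; BP_Pawn is a pawn Blueprint that scores a point whenever it begins overlapping a BP_ActorWork13 actor.
; It increments Score on the BP_MyGI game instance, then passes the new value to AddScore on player 0's BP_MyHUD.
; A sequence calls the parent overlap handler afterwards, even when a cast fails.
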(event `self.ReceiveActorBeginOverlap`
  (params (OtherActor :type "Actor Object Reference"))
  (`|ExecutionSequence`
    (:`then_0`
      (cast `/Game/BP_ActorWork13` OtherActor)
      (bind _asbp_my_gi (cast `/Game/BP_MyGI` (`GameplayStatics.GetGameInstance`)))
      (bind _result (`/Engine/EditorBlueprintResources/StandardMacros.IncrementInt` (`/Game/BP_MyGI.Score` _asbp_my_gi))
        (:`  `
          (bind _output_get (set `/Game/BP_MyGI.Score` _result _asbp_my_gi))
          (bind _asbp_my_hud (cast `/Game/BP_MyHUD` (`PlayerController.GetHUD` (`GameplayStatics.GetPlayerController` 0))))
          (`/Game/BP_MyHUD.AddScore` _asbp_my_hud _output_get))))
    (:`then_1`
      (`parent.ReceiveActorBeginOverlap` OtherActor))))

(fn `UserConstructionScript`)