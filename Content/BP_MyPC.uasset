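; Player controller that adds an Enhanced Input mapping context and drives the possessed BP_PawnClass, which it caches on Possess.
; Move input offsets the pawn along control-rotation forward and right vectors, scaled by the pawn's MovementMultiplier, without sweep or delta-time scaling.
; Jump shifts the pawn along its up vector by JumpMultiplier on press and back down on release, with no physics.
; Look input feeds controller yaw and pitch.
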(event `self.ReceiveBeginPlay`
  (bind _returnvalue (pcsubsystem `EnhancedInputLocalPlayerSubsystem` self))
  (`/Engine/EditorBlueprintResources/StandardMacros.IsValid` _returnvalue
    (:`Is Valid`
      (`EnhancedInputSubsystemInterface.AddMappingContext` _returnvalue "/Game/Input/IM_Sample.IM_Sample" 0 (struct)))))

(event `EnhancedInput|/Game/Input/IA_Move2`
  (params (ActionValue :type "Vector2D Structure") (ElapsedSeconds :type "Float (double-precision)") (TriggeredSeconds :type "Float (double-precision)") (InputAction :type "InputAction Object Reference" :default "/Game/Input/IA_Move2.IA_Move2"))
  (bind (_returnvalue_roll _returnvalue_pitch _returnvalue_yaw) (`KismetMathLibrary.BreakRotator` (`self.GetControlRotation`)))
  (bind (_returnvalue_roll_2 _returnvalue_pitch_2 _returnvalue_yaw_2) (`KismetMathLibrary.BreakRotator` (`self.GetControlRotation`)))
  (bind _movementmultiplier (`/Game/BP_PawnClass.MovementMultiplier` (`self.PosssedPawn`)))
  (:`Triggered`
    (`self.K2_AddActorWorldOffset` (`GameplayStatics.GetPlayerPawn` 0) (* (* ActionValue_Y _movementmultiplier) (`KismetMathLibrary.GetForwardVector` (`KismetMathLibrary.MakeRotator` 0.0 0.0 _returnvalue_yaw))) false false)
    (`self.K2_AddActorWorldOffset` (`GameplayStatics.GetPlayerPawn` 0) (* (* ActionValue_X _movementmultiplier) (`KismetMathLibrary.GetRightVector` (`KismetMathLibrary.MakeRotator` _returnvalue_roll_2 0.0 _returnvalue_yaw_2))) false false)))

(event `self.ReceivePossess`
  (params (PossessedPawn :type "Pawn Object Reference"))
  (bind _asbp_pawn_class (cast `/Game/BP_PawnClass` PossessedPawn)
    (:`then`
      (set `self.PosssedPawn` _asbp_pawn_class))
    (:`CastFailed`
      (set `self.PosssedPawn` _asbp_pawn_class))))

(event `EnhancedInput|/Game/Input/IA_Jump2`
  (params (ActionValue :type Boolean) (ElapsedSeconds :type "Float (double-precision)") (TriggeredSeconds :type "Float (double-precision)") (InputAction :type "InputAction Object Reference" :default "/Game/Input/IA_Jump2.IA_Jump2"))
  (bind _posssedpawn (`self.PosssedPawn`))
  (:`Started`
    (set `self.isStart` 1.0)
    (`self.K2_AddActorWorldOffset` (`GameplayStatics.GetPlayerPawn` 0) (* (* (`SceneComponent.GetUpVector` (`Actor.RootComponent` _posssedpawn)) (`/Game/BP_PawnClass.JumpMultiplier` _posssedpawn)) (`self.isStart`)) false false :!label _label))
  (:`Completed`
    (set `self.isStart` -1.0)
    (goto _label)))

(event `EnhancedInput|/Game/Input/IA_Look2`
  (params (ActionValue :type "Vector2D Structure") (ElapsedSeconds :type "Float (double-precision)") (TriggeredSeconds :type "Float (double-precision)") (InputAction :type "InputAction Object Reference" :default "/Game/Input/IA_Look2.IA_Look2"))
  (:`Triggered`
    (`Pawn.AddControllerYawInput` (`GameplayStatics.GetPlayerPawn` 0) ActionValue_X)
    (`Pawn.AddControllerPitchInput` (`GameplayStatics.GetPlayerPawn` 0) ActionValue_Y)))

(fn `UserConstructionScript`)