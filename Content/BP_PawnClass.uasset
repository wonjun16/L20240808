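; BP_PawnClass is a pawn that lets the player transfer possession to another BP_PawnClass pawn it overlaps.
; Overlap events maintain an IsOverlap flag, and both overlap begin and the MyInteract Enhanced Input action run the same check for input plus overlap.
; On success, the player controller possesses the overlapped pawn and adds the IM_Sample mapping context through the Enhanced Input subsystem.
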(event `EnhancedInput|/Game/Input/MyInteract`
  (params (ActionValue :type Boolean) (ElapsedSeconds :type "Float (double-precision)") (TriggeredSeconds :type "Float (double-precision)") (InputAction :type "InputAction Object Reference" :default "/Game/Input/MyInteract.MyInteract"))
  (:`Triggered`
    (if (and ActionValue (`self.isOverlap`)) :!label _label
      (bind _asbp_pawn_class (cast `/Game/BP_PawnClass` (stale `self.ReceiveActorBeginOverlap` OtherActor)))
      (bind _output_get (set `self.OverlapedPawn` _asbp_pawn_class))
      (bind _asplayer_controller (cast `PlayerController` (`self.GetController`)))
      (bind _returnvalue (pcsubsystem `EnhancedInputLocalPlayerSubsystem` _asplayer_controller))
      (`/Engine/EditorBlueprintResources/StandardMacros.IsValid` _returnvalue
        (:`Is Valid`
          (`Controller.Possess` _asplayer_controller _output_get)
          (`EnhancedInputSubsystemInterface.AddMappingContext` _returnvalue "/Game/Input/IM_Sample.IM_Sample" 0 (struct)))))))

(event `self.ReceiveActorBeginOverlap`
  (params (OtherActor :type "Actor Object Reference"))
  (set `self.isOverlap` true)
  (goto _label))

(event `self.ReceiveActorEndOverlap`
  (params (OtherActor :type "Actor Object Reference"))
  (set `self.isOverlap` false))

(fn `UserConstructionScript`)